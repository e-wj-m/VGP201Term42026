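; Enemy AI character that takes damage, fires bullets and awards score when killed.
; A health component starts at full on BeginPlay, and AnyDamage feeds DamageEnemy, which on death adds a point through BP_MainSceneGameMode and destroys the actor.
; FireAtTarget spawns BP_BaseBullet at the player pawn's location, using the gun spawn point's rotation, then calls FireAtTarget again with no delay.
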(event Custom|FireAtTarget
  (Game|SpawnActorfromClass "/Game/Blueprints/Game/Projectiles/BP_BaseBullet.BP_BaseBullet_C" (Math|Transform|MakeTransform (Transformation|GetActorLocation (Game|Player|GetPlayerPawn 0)) (Transformation|GetWorldRotation (Variables|Default|GetGunSpawnPoint)) "1.000000,1.000000,1.000000") "Undefined" "MultiplyWithRoot" 0 0)
  (CallFunction|FireatTarget))

(event EventBeginPlay
  (Default|Init (Variables|Default|GetAC_HealthComponent) 5e+01 0.0 5e+01))

(event Collision|EventActorBeginOverlap
  (params (OtherActor :type Actor%20Object%20Reference)))

(event EventTick
  (params (DeltaSeconds :type Float%20%28single-precision%29)))

(event Game|Damage|EventAnyDamage
  (params (Damage :type Float%20%28single-precision%29) (DamageType :type Damage%20Type%20Object%20Reference) (InstigatedBy :type Controller%20Object%20Reference) (DamageCauser :type Actor%20Object%20Reference))
  (CallFunction|DamageEnemy Damage)
  (Utilities|String|LogString "Enemy should be taking damage"))

(fn ConstructionScript)

(fn DamageEnemy
  (params (DamageValue :type Float%20%28double-precision%29))
  (bind _ac_healthcomponent (Variables|Default|GetAC_HealthComponent))
  (Default|Damage _ac_healthcomponent DamageValue)
  (if (Default|IsDead _ac_healthcomponent)
    (bind _asbp_main_scene_game_mode (Utilities|Casting|CastToBP_MainSceneGameMode (Game|GetGameMode)))
    (Default|AddScore _asbp_main_scene_game_mode 1)
    (Actor|DestroyActor)))