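; BP_ScoreManager keeps the player's score and shows it as the kill count in the game menu.
; AddToScore ignores negative amounts, adds the rest to Score, then calls UpdateScore.
; UpdateScore reaches the menu widget through BP_MainSceneGameMode's GameMenuRef and passes the score to SetKillCount.
; BeginPlay waits briefly before pushing the initial score to the menu.
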(event EventBeginPlay
  (Utilities|FlowControl|Delay 1.0)
  (CallFunction|AddtoScore)
  (CallFunction|UpdateScore))

(event Collision|EventActorBeginOverlap
  (params (OtherActor :type Actor%20Object%20Reference)))

(event EventTick
  (params (DeltaSeconds :type Float%20%28single-precision%29)))

(fn ConstructionScript)

(fn UpdateScore
  (bind _asbp_main_scene_game_mode (Utilities|Casting|CastToBP_MainSceneGameMode (Game|GetGameMode)))
  (Default|SetKillCount (Variables|/Game/Blueprints/Game/Managers/BP_MainSceneGameMode.BP_MainSceneGameMode_C|GetGameMenuRef _asbp_main_scene_game_mode) (Variables|Default|GetScore)))

(fn AddtoScore
  (params (Amount :type Integer))
  (Variables|Default|SetScore (+ (Variables|Default|GetScore) (Math|Integer|Clamp(Integer) Amount 0 2147483647)))
  (CallFunction|UpdateScore))