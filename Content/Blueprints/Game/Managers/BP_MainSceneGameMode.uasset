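; BP_MainSceneGameMode is the main scene's game mode, which sets up the game menu, input and score manager on BeginPlay.
; It creates WBP_GameMenu, switches to game-only input without a cursor, and pushes GameTimer to the menu once.
; It then spawns BP_ScoreManager, stores the reference and adds an initial point.
; The timer is unfinished: Tick only runs a Delay, and the GameTimer addition is unconnected.
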(event Custom|CustomEvent)

(event EventTick
  (params (DeltaSeconds :type Float%20%28single-precision%29))
  (Utilities|FlowControl|Delay 0.2))

(event EventBeginPlay
  (Development|PrintString "Hello YA BITCH")
  (Development|PrintString "SpawningBP_MainSceneGameMode")
  (CallFunction|SpawnGameMenu)
  (CallFunction|SetInputtoGame)
  (CallFunction|UpdateTimer)
  (bind _returnvalue (Game|SpawnActorfromClass "/Game/Blueprints/Game/Managers/BP_ScoreManager.BP_ScoreManager_C" (Math|Transform|MakeTransform "0, 0, 0" "0, 0, 0" "1.000000,1.000000,1.000000") "Undefined" "MultiplyWithRoot" 0 0))
  (bind _output_get (Variables|Default|SetScoreManagerRef _returnvalue))
  (Default|AddtoScore _output_get 1))

(fn ConstructionScript)

(fn SpawnGameMenu
  (bind _returnvalue (UserInterface|CreateWidget "/Game/Blueprints/Game/GUI/WBP_GameMenu.WBP_GameMenu_C"))
  (bind _output_get (Variables|Default|SetGameMenuRef _returnvalue))
  (UserInterface|Viewport|AddtoViewport _output_get 0))

(fn SetInputtoGame
  (bind _returnvalue (Game|GetPlayerController 0))
  (Input|SetInputModeGameOnly _returnvalue false)
  (Variables|/Script/Engine.PlayerController|SetbShowMouseCursor _returnvalue false))

(fn UpdateTimer
  (Default|SetTimer (Variables|Default|GetGameMenuRef) (Variables|Config|GetGameTimer)))