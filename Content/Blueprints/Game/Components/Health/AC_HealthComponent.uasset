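; Health component that stores an actor's health between minimum and maximum limits, with damage, heal, reset and status queries.
; Damage and Heal reject non-positive amounts and pass through SetHealth, which clamps; HealFull and Death reuse them with MaxHealth.
; Init calls SetHealth before assigning the new limits, so clamping uses the previous ones.
; BeginPlay runs a debug damage-and-heal sequence, printing health along the way.
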(event EventBeginPlay
  (CallFunction|PrintHealth)
  (CallFunction|Damage 25.0)
  (CallFunction|PrintHealth)
  (CallFunction|Heal 15.0)
  (CallFunction|PrintHealth))

(fn Reset
  (Variables|Default|SetHealth (Variables|Default|GetMaxHealth)))

(fn GetHealth
  (return (Variables|Default|GetHealth)))

(fn SetHealth
  (params (NewHealth :type Float%20%28double-precision%29))
  (bind _output_get (Variables|Default|SetHealth (CallFunction|ClampHealth NewHealth)))
  (return _output_get))

(fn PrintHealth
  (Development|PrintString (Utilities|String|ToString(Float) (CallFunction|GetHealth))))

(fn ClampHealth
  (params (Value :type Float%20%28double-precision%29))
  (return (Math|Float|Clamp(Float) Value (Variables|Default|GetMinHealth) (Variables|Default|GetMaxHealth))))

(fn Damage
  (params (DamageAmount :type Float%20%28double-precision%29))
  (if (> DamageAmount 0.0)
    (CallFunction|SetHealth (- (CallFunction|GetHealth) DamageAmount))
    (else
      (Development|PrintString "Damage must be positive YA DING DONG"))))

(fn Heal
  (params (HealAmount :type Float%20%28double-precision%29))
  (if (> HealAmount 0.0)
    (CallFunction|SetHealth (+ (CallFunction|GetHealth) HealAmount))
    (else
      (Development|PrintString "Heal amount must be positive YA DING DONG"))))

(fn HealFull
  (CallFunction|Heal (Variables|Default|GetMaxHealth)))

(fn Death
  (CallFunction|Damage (Variables|Default|GetMaxHealth)))

(fn GetNormalizedHealth
  (return (Math|Float|Clamp(Float) (/ (CallFunction|GetHealth) (Variables|Default|GetMaxHealth)))))

(fn IsDead
  (return (<= (CallFunction|GetHealth) (Variables|Default|GetMinHealth))))

(fn Init
  (params (Health :type Float%20%28double-precision%29) (MinHealth :type Float%20%28double-precision%29) (MaxHealth :type Float%20%28double-precision%29))
  (CallFunction|SetHealth Health)
  (Variables|Default|SetMinHealth MinHealth)
  (Variables|Default|SetMaxHealth MaxHealth))