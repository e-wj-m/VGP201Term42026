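; BP_Rifle is a rifle weapon Blueprint that extends a parent gun class with hitscan damage.
; OnGunShoot calls the parent, line traces the Visibility channel between the given points, then applies the Damage value to the hit actor.
; The trace draws timed debug lines and prints the hit actor's name.
; GetDamage returns a fixed value; the event graph and construction script add no logic.
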(event EventBeginPlay
  (|CallParentFunction) ; This node is disabled and will not be called.\nDrag off pins to build functionality.
)

(event Collision|EventActorBeginOverlap
  (params (OtherActor :type Actor%20Object%20Reference))
  (|CallParentFunction OtherActor) ; This node is disabled and will not be called.\nDrag off pins to build functionality.
)

(event EventTick
  (params (DeltaSeconds :type Float%20%28single-precision%29))
  (|CallParentFunction DeltaSeconds) ; This node is disabled and will not be called.\nDrag off pins to build functionality.
)

(fn ConstructionScript
  (|CallParentFunction))

(fn OnGunShoot
  (params (Start%20Pos :type Vector :default "0, 0, 0") (End%20Pos :type Vector :default "0, 0, 0"))
  (|CallParentFunction Start%20Pos End%20Pos)
  (bind _outhit (Collision|LineTraceByChannel Start%20Pos End%20Pos "TraceTypeQuery1" false 0 "ForDuration" true "(R=1.000000,G=0.000000,B=0.000000,A=1.000000)" "(R=0.000000,G=1.000000,B=0.000000,A=1.000000)" 3.0))
  (Development|PrintString (Utilities|GetDisplayName (.HitActor (Collision|BreakHitResult _outhit))))
  (Game|Damage|ApplyDamage (.HitActor (Collision|BreakHitResult _outhit)) (Variables|Default|GetDamage) 0 0))

(fn GetDamage
  (return 5e+01))