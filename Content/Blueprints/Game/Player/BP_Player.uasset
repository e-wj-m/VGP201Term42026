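; Player character with movement, look, jump, gun firing and health.
; On BeginPlay it attaches a spawned StartingGun and initialises ACHealthComponent.
; The Shoot axis fires through BPI_Gun along the camera's forward vector to the gun's range, using a fire-rate Delay before each shot, while left mouse separately spawns a projectile from the gun.
; Damage updates the health bar through BP_MainSceneGameMode, which also receives the game-over call on death.
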(event EventBeginPlay
  ;[0.15 0.1391 0 0.5] Debug
  (Development|PrintString "Spawning Player" true true "(R=1.000000,G=0.185596,B=0.000000,A=1.000000)" 5.0)
  (CallFunction|SpawnGun (Variables|Default|GetStartingGun))
  (Default|Init (Variables|Default|GetAC_HealthComponent) 1e+02 0.0 1e+02)
  (CallFunction|UpdateHealthBar))

(event Game|Damage|EventAnyDamage
  (params (Damage :type Float%20%28single-precision%29) (DamageType :type Damage%20Type%20Object%20Reference) (InstigatedBy :type Controller%20Object%20Reference) (DamageCauser :type Actor%20Object%20Reference))
  ;[1 0.1856 0] Damage the Player Entity
  (CallFunction|OnDamagePlayer Damage))

(event Input|ActionEvents|InputActionJump
  (params (Key :type Key%20Structure :default "None"))
  ;[0 0.04452 0.15 0.5] Jump Logic
  (:Pressed
    (Character|Jump)))

(event Input|AxisEvents|InputAxisForwardsBackwardsMovement
  (params (AxisValue :type Float%20%28single-precision%29))
  ;[0 0.02832 0.15 0.5] Movement Logic
  (Pawn|Input|AddMovementInput (Transformation|GetActorForwardVector) AxisValue false))

(event Input|AxisEvents|InputAxisHorizontalCamera
  (params (AxisValue :type Float%20%28single-precision%29))
  ;[0.006665 0.01009 0.15 0.5] Camera Logic
  (Pawn|Input|AddControllerYawInput AxisValue))

(event Input|AxisEvents|InputAxisVerticalCamera
  (params (AxisValue :type Float%20%28single-precision%29))
  ;[0.006665 0.01009 0.15 0.5] Camera Logic
  (Pawn|Input|AddControllerPitchInput AxisValue))

(event Input|AxisEvents|InputAxisShoot
  (params (AxisValue :type Float%20%28single-precision%29))
  ;[0.15 0 0.002117 0.5] Firing Logic
  (if (> AxisValue 0.0)
    (Utilities|PlayerFiring)))

(event Input|AxisEvents|InputAxisLeftwardsRightwardsMovement
  (params (AxisValue :type Float%20%28single-precision%29))
  ;[0 0.02832 0.15 0.5] Movement Logic
  (Pawn|Input|AddMovementInput (Transformation|GetActorRightVector) AxisValue false))

(event Input|MouseEvents|LeftMouseButton
  (params (Key :type Key%20Structure :default "None"))
  ;[1 0 0.06333] Projectile Logic
  (:Pressed
    (Utilities|ProjectileFiring)))

(fn ConstructionScript)

(fn SpawnGun
  (params (GunToSpawn :type Actor%20Class%20Reference))
  (bind _returnvalue (Game|SpawnActorfromClass GunToSpawn (Math|Transform|MakeTransform "0, 0, 0" "0, 0, 0" "0.750000,0.750000,0.750000") "Undefined" "MultiplyWithRoot" 0 0))
  (bind _output_get (Variables|Default|SetGunRef _returnvalue))
  (Transformation|AttachComponentToComponent _output_get (Variables|Default|GetGunSpawnPoint) "None" "SnapToTarget" "SnapToTarget" "KeepRelative" true)
  (bind _asbpi_gun (Utilities|Casting|CastToBPI_Gun _output_get)
    (:then
      (Variables|Default|SetGunInterfaceRef _asbpi_gun))
    (:CastFailed
      _))
  (return _output_get))

(fn CalculateShoot
  (bind _camera (Variables|Default|GetCamera))
  (bind _returnvalue (Transformation|GetWorldLocation _camera))
  (bind _range (Class|BPIGun|GetRange(Message) (Utilities|ToObject(Interface) (Variables|Default|GetGunInterfaceRef))))
  (return _returnvalue (+ _returnvalue (* (Math|Vector|GetForwardVector _camera) _range))))

(fn OnDamagePlayer
  (params (Amount :type Float%20%28double-precision%29))
  (bind _ac_healthcomponent (Variables|Default|GetAC_HealthComponent))
  (Default|Damage _ac_healthcomponent Amount)
  (CallFunction|UpdateHealthBar)
  (if (Default|IsDead _ac_healthcomponent)
    (bind _asbp_main_scene_game_mode (Utilities|Casting|CastToBP_MainSceneGameMode (Game|GetGameMode)))
    (Default|CallGameOver _asbp_main_scene_game_mode)))

(fn UpdateHealthBar
  (bind _asbp_main_scene_game_mode (Utilities|Casting|CastToBP_MainSceneGameMode (Game|GetGameMode)))
  (Default|SetHealthBar (Variables|/Game/Blueprints/Game/Managers/BP_MainSceneGameMode.BP_MainSceneGameMode_C|GetGameMenuRef _asbp_main_scene_game_mode) (Default|GetNormalizedHealth (Variables|Default|GetAC_HealthComponent))))