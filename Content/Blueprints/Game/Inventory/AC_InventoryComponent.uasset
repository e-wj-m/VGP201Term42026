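; AC_InventoryComponent is an inventory component that holds a fixed-size item array and displays it through a grid widget.
; On BeginPlay it adds the default input mapping context, creates the inventory widget, sizes Items to InventorySize and refreshes the widget from itself.
; The inventory input action only opens the widget: it adds it to the viewport, shows the cursor and switches input to UI-only.
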(event Input|EnhancedActionEvents|EnhancedInputActionIA_Inventory
  (params (ActionValue :type Boolean) (ElapsedSeconds :type Float%20%28double-precision%29) (TriggeredSeconds :type Float%20%28double-precision%29) (InputAction :type Input%20Action%20Object%20Reference :default "/Game/Blueprints/Game/Input/Actions/IA_Inventory.IA_Inventory"))
  (bind _returnvalue (Game|GetPlayerController 0))
  (bind _inventory_reference (Variables|Default|GetInventory%20Reference))
  (bind _inventory_reference_2 (Variables|Default|GetInventory%20Reference))
  ;[0.15 0.08495 0.000583 0.5] Inventory Action (Tab Key)
  (if (not (UserInterface|Viewport|IsinViewport _inventory_reference))
    (UserInterface|Viewport|AddtoViewport _inventory_reference 0)
    (Variables|/Script/Engine.PlayerController|SetbShowMouseCursor _returnvalue true)
    (Input|SetInputModeUIOnly _returnvalue _inventory_reference_2 "DoNotLock" false)
    (Variables|/Script/UMG.UserWidget|SetbIsFocusable _inventory_reference_2 true)))

(event EventBeginPlay
  ;[0.15 0.04431 0.1464 0.5] Begin Play
  (Input|AddMappingContext (PlayerController|LocalPlayerSubsystems|GetEnhancedInputLocalPlayerSubsystem (Game|GetPlayerController 0)) "/Game/Blueprints/Game/Input/IMC_Default.IMC_Default" 0 "(bIgnoreAllPressedKeysUntilRelease=True,bForceImmediately=False,bNotifyUserSettings=False)")
  (bind _returnvalue (UserInterface|CreateWidget "/Game/Blueprints/Game/Inventory/W_InventoryGrid.W_InventoryGrid_C"))
  (Variables|Default|SetInventory%20Reference _returnvalue)
  (Utilities|Array|Resize (Variables|Default|GetItems) (Variables|Default|GetInventorySize))
  (Default|RefreshInventory (Variables|Default|GetInventory%20Reference) self))