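; BP_Player is the player character, handling movement, jumping, camera look and gun firing.
; On BeginPlay it spawns the starting gun and snaps it to the gun spawn point.
; Holding Shoot calls PlayerFiring, whose Delay on the gun's FireRate paces each shot.
; Each shot passes the gun's OnGunShoot a start and end point projected from the camera's forward vector over the gun's Range.
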(event EventBeginPlay
  ;[0.15 0.15 0.15 0.5] Debug
  (Development|PrintString "Spawning Player" true true "(R=1.000000,G=0.185596,B=0.000000,A=1.000000)" 5.0)
  (CallFunction|SpawnGun (Variables|Default|GetStartingGun)))

(event Input|ActionEvents|InputActionJump
  (params (Key :type Key%20Structure :default "None"))
  ;[0.15 0.15 0.15 0.5] Jump Logic
  (:Pressed
    (Character|Jump)))

(event Input|AxisEvents|InputAxisForwardsBackwardsMovement
  (params (AxisValue :type Float%20%28single-precision%29))
  ;[0.15 0.15 0.15 0.5] Movement Logic
  (Pawn|Input|AddMovementInput (Transformation|GetActorForwardVector) AxisValue false))

(event Input|AxisEvents|InputAxisHorizontalCamera
  (params (AxisValue :type Float%20%28single-precision%29))
  ;[0.15 0.15 0.15 0.5] Camera Logic
  (Pawn|Input|AddControllerYawInput AxisValue))

(event Input|AxisEvents|InputAxisVerticalCamera
  (params (AxisValue :type Float%20%28single-precision%29))
  ;[0.15 0.15 0.15 0.5] Camera Logic
  (Pawn|Input|AddControllerPitchInput AxisValue))

(event Input|AxisEvents|InputAxisShoot
  (params (AxisValue :type Float%20%28single-precision%29))
  ;[0.15 0.15 0.15 0.5] Firing Logic
  (if (> AxisValue 0.0)
    (Utilities|PlayerFiring)))

(event Input|AxisEvents|InputAxisLeftwardsRightwardsMovement
  (params (AxisValue :type Float%20%28single-precision%29))
  ;[0.15 0.15 0.15 0.5] Movement Logic
  (Pawn|Input|AddMovementInput (Transformation|GetActorRightVector) AxisValue false))

(fn ConstructionScript)

(fn SpawnGun
  (params (GunToSpawn :type BP%20Gun%20Class%20Reference))
  (bind _returnvalue (Game|SpawnActorfromClass GunToSpawn (Math|Transform|MakeTransform "0, 0, 0") "Undefined" "MultiplyWithRoot" 0 0))
  (bind _output_get (Variables|Default|SetGunRef _returnvalue))
  (Transformation|AttachComponentToComponent _output_get (Variables|Default|GetGunSpawnPoint) "None" "SnapToTarget" "SnapToTarget" "SnapToTarget" true)
  (return _output_get))

(fn CalculateShoot
  (bind _camera (Variables|Default|GetCamera))
  (bind _returnvalue (Transformation|GetWorldLocation _camera))
  (return _returnvalue (+ _returnvalue (* (Math|Vector|GetForwardVector _camera) (Variables|/Game/Blueprints/Weapons/BP_Gun.BP_Gun_C|GetRange (Variables|Default|GetGunRef))))))